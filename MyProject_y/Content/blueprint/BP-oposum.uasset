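; BP-oposum is a side-scrolling opossum enemy that patrols between two referenced point actors, set as InterpToMovement control points in the construction script.
; On each movement reversal it flips its X scale from velocity direction to face its travel.
; When BP-kitty overlaps its Box while falling, it launches the kitty upward, spawns an enemy-death BPdust effect and destroys itself.
; Otherwise, overlapping damages the kitty.
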(event `self.InterpToMovement.OnInterpToReverse`
  (params (ImpactResult :type "HitResult Structure (by ref)") (Time :type "Float (single-precision)"))
  ;[1 1 1] HandleRotation
  (`/Engine/EditorBlueprintResources/StandardMacros.CompareFloat` (.x (`self.GetVelocity`))
    (:`>`
      (`self.SetActorRelativeScale3D` (1.0 1.0 1.0)))
    (:`<`
      (`self.SetActorRelativeScale3D` (-1.0 1.0 1.0)))))

(event `self.Box.OnComponentBeginOverlap`
  (params (OverlappedComponent :type "PrimitiveComponent Object Reference") (OtherActor :type "Actor Object Reference") (OtherComp :type "PrimitiveComponent Object Reference") (OtherBodyIndex :type Integer) (bFromSweep :type Boolean) (SweepResult :type "HitResult Structure (by ref)"))
  ;[1 1 1] Comment
  (bind _asbp_kitty (cast `/Game/paperzd/character/BP-kitty` OtherActor))
  (bind (_velocity_x _velocity_y _velocity_z) (`KismetMathLibrary.BreakVector` (`MovementComponent.Velocity` (`Character.CharacterMovement` _asbp_kitty))))
  (if (< _velocity_z 0.0)
    (`Character.LaunchCharacter` _asbp_kitty (0.0 0.0 800.0) false false)
    (`|SpawnActorFromClass` "/Game/actors/BP-dust.BP-dust_C" (`self.GetTransform`) "Undefined" "OverrideRootScale" null "/Game/assets/flipbooks/enemydeath/fb-enemy-deadth.fb-enemy-deadth" null)
    (`self.K2_DestroyActor`)
    (else
      (`GameplayStatics.ApplyDamage` OtherActor 15.0))))

(fn `UserConstructionScript`
  (set `InterpToMovementComponent.ControlPoints` (`|MakeArray` (make `InterpControlPoint` (`self.K2_GetActorLocation` (`self.firstpoint`)) false) (make `InterpControlPoint` (`self.K2_GetActorLocation` (`self.secondpoint`)) false)) (`self.InterpToMovement`)))